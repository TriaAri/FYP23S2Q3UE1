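; Test boid actor for flocking, with only the alignment rule present, seeded with a random XY velocity.
; Flock stores Align's steering, the clamped difference between average neighbour velocity and its own, as Acceleration.
; MoveBoid adds Velocity to Position and moves the Cube, never applying Acceleration.
; Edges only caps positive X, and nothing here calls MoveBoid, Flock or Edges.
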(event `self.ReceiveBeginPlay`
  (set `self.position` (`SceneComponent.K2_GetComponentLocation` (`self.Cube`)))
  (set `self.velocity` (`KismetMathLibrary.MakeVector` (`KismetMathLibrary.RandomFloatInRange` -10.0 10.0) (`KismetMathLibrary.RandomFloatInRange` -10.0 10.0))))

(fn `Align`
  (params (boids :type "Array of /Game/Test/Blueprints/BP_Boid Object Reference"))
  (returns (steeringValue :type "Vector Structure"))
  (locals (steering :type "Vector Structure") (perceptionRadius :type "Float (double-precision)" :default 100.0) (total :type Integer) (distance :type "Float (double-precision)"))
  (bind (_maxforce_x _maxforce_y _maxforce_z) (`KismetMathLibrary.BreakVector` (`self.maxForce`)))
  (bind _steering (`local.steering`))
  (for _array_element boids
    (set `local.distance` (`KismetMathLibrary.Vector_Distance` (`self.position`) (`/Game/Test/Blueprints/BP_Boid.position` _array_element)))
    (if (and (!= self _array_element) (< (`local.distance`) (`local.perceptionRadius`)))
      (set `local.steering` (+ (`local.steering`) (`/Game/Test/Blueprints/BP_Boid.velocity` _array_element)))
      (`/Engine/EditorBlueprintResources/StandardMacros.IncrementInt` (`local.total`))))
  (if (> (`local.total`) 0)
    (bind _output_get (set `local.steering` (/ _steering (`local.total`))))
    (bind _output_get_2 (set `local.steering` (- _output_get (`self.velocity`))))
    (return (`KismetMathLibrary.ClampVectorSize` _output_get_2 0.0 _maxforce_z))
    (else
      (return _steering))))

(fn `Edges`
  (bind (_position_x _position_y _position_z) (`KismetMathLibrary.BreakVector` (`self.position`)))
  (if (> _position_x 4000.0)
    (`KismetMathLibrary.Vector_Set` (`self.position`) 4000.0 _position_y _position_z)))

(fn `Flock`
  (params (boids :type "Array of /Game/Test/Blueprints/BP_Boid Object Reference"))
  (locals (alignment :type "Vector Structure"))
  (bind _steeringvalue (`self.Align` boids))
  (bind _output_get (set `local.alignment` _steeringvalue))
  (set `self.acceleration` _output_get))

(fn `MoveBoid`
  (bind _output_get (set `self.position` (+ (`self.position`) (`self.velocity`))))
  (`KismetSystemLibrary.PrintString` (`KismetStringLibrary.Conv_VectorToString` _output_get))
  (`SceneComponent.K2_SetWorldLocation` (`self.Cube`) _output_get false false))

(fn `UserConstructionScript`)
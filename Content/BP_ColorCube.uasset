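; BP_ColorCube is a cube actor that prepares a dynamic material and a hidden UI widget.
; The Construction Script creates a dynamic instance of M_ColorCube on the ColorCube component and stores it in DynamicMaterial.
; BeginPlay enables input for the first player controller, then creates WBP_UI, adds it to the viewport and hides it.
; No logic here changes the color or reveals the widget.
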(event `self.ReceiveBeginPlay`
  (bind _returnvalue (`GameplayStatics.GetPlayerController` 0))
  (bind _widget (`self.Widget`))
  (`self.EnableInput` _returnvalue)
  (bind _returnvalue_2 (`|CreateWidget` "/Game/WBP_UI.WBP_UI_C" _returnvalue))
  (set `self.Widget` _returnvalue_2)
  (`UserWidget.AddToViewport` _widget 0)
  (`Widget.SetVisibility` _widget "Hidden"))

(fn `UserConstructionScript`
  (bind _returnvalue (`PrimitiveComponent.CreateDynamicMaterialInstance` (`self.ColorCube`) 0 "/Game/M_ColorCube.M_ColorCube" "None"))
  (set `self.Dynamic Material` _returnvalue))